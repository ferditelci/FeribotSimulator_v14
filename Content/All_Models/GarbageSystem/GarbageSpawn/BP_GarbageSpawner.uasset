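; BP_GarbageSpawner is a spawner actor that keeps one randomly chosen piece of garbage present at its location.
; A delayed Tick periodically calls AttemptToSpawn, which spawns only when CurrentGarbage is invalid.
; SpawnGarbage picks a class from GarbageToSpawn, spawns it owned by the spawner, then randomizes its yaw.
; The Respawn event clears the tracked reference and retries after a delay, though Tick polling can refill it sooner.
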(event EventRespawn
  (Variables|Default|SetCurrentGarbage 0)
  (Utilities|FlowControl|Delay 2.0)
  (CallFunction|AttempttoSpawn))

(event EventTick
  (params (DeltaSeconds :type Float%20%28single-precision%29))
  (Utilities|FlowControl|Delay 1.0)
  (CallFunction|AttempttoSpawn))

(fn ConstructionScript)

(fn AttempttoSpawn
  (Utilities|IsValid (Variables|Default|GetCurrentGarbage)
    (:Is%20Not%20Valid
      (CallFunction|SpawnGarbage))))

(fn SpawnGarbage
  (bind _returnvalue (Game|SpawnActorfromClass (Utilities|Array|Get(acopy) (Variables|Default|GetGarbageToSpawn) (Math|Random|RandomIntegerinRange 0 (Utilities|Array|LastIndex (Variables|Default|GetGarbageToSpawn)))) (Math|Transform|MakeTransform (Transformation|GetActorLocation) (Transformation|GetActorRotation)) "AdjustIfPossibleButAlwaysSpawn" self 0))
  (bind _output_get (Variables|Default|SetCurrentGarbage _returnvalue))
  (Utilities|IsValid _output_get
    (:Is%20Valid
      (Transformation|SetActorRotation _output_get (Math|Rotator|MakeRotator 0.0 0.0 (Math|Random|RandomFloatinRange 0.0 3.6e+02))))))